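; Player-driven Mars rover vehicle pawn with switchable first-person and zoomable chase cameras, toggleable lights, brake lights and wheel dust.
; Tick feeds input to VehicleMovement, adding force for quicker acceleration and braking, using box traces for ground checks.
; Middle-wheel suspension is faked: line traces set AnimBP offsets and move wheel collision meshes to match.
; Stabilizing torque resists rolling; a stuck, overturned rover fades out and teleports to world origin.
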(event EventTick
  (params (DeltaSeconds :type Float%20%28single-precision%29))
  ;[1 0.06514 0] Event Tick
  (Utilities|FlowControl|Sequence
    (:then_0
      (|DetectWhetherCarisonGround)
      (|HelpPreventCarfromRolling)
      (|Respawnifrolledover))
    (:then_1
      (|SmoothenCameraArmLength)
      (|ArtificialMiddleWheelSpring&Collision))
    (:then_2
      ;[1 0.8922 0] Driving Input
      ;;[1 1 1] Forward & Reverse
      (|ApplyThrottle))
    (:then_3
      (|ActivateDustParticleswhenrearwheelstouchground))
    (:then_4
      ;;[1 1 1] Brake
      (|BrakingToggle)
      (|BrakeLightToggle))))

(event EventBeginPlay
  ;[1 0 0] Begin Play
  (|GetAccesstoAnimBP)
  (Variables|Default|SetWheelCollision_ML_Location (Variables|/Script/Engine.SceneComponent|GetRelativeLocation (Variables|Default|GetWheel_Collision_L))) ; Store the relative Wheel Collision location before any animation so we can use it to drive the animation each tick
  (Variables|Default|SetWheelCollision_MR_Location (Variables|/Script/Engine.SceneComponent|GetRelativeLocation (Variables|Default|GetWheel_Collision_R))))

(event Input|ActionEvents|InputActionTorch
  (params (Key :type Key%20Structure))
  ;[1 0.8922 0] Driving Input
  ;;[1 1 1] Torch
  (:Pressed
    (CallFunction|ToggleTorch)))

(event Input|ActionEvents|InputActionBrake
  (params (Key :type Key%20Structure))
  ;[1 0.8922 0] Driving Input
  ;;[1 1 1] Brake
  (:Pressed
    (Variables|Default|SetBraking true))
  (:Released
    (Variables|Default|SetBraking false)))

(event Input|AxisEvents|InputAxisMoveRight
  (params (AxisValue :type Float%20%28single-precision%29))
  ;[1 0.8922 0] Driving Input
  ;;[1 1 1] Steering
  (Class|WheeledVehicleMovementComponent|SetSteeringInput (Variables|Default|GetVehicleMovement) AxisValue))

(event Input|AxisEvents|InputAxisMoveForward
  (params (AxisValue :type Float%20%28single-precision%29))
  ;[1 0.8922 0] Driving Input
  ;;[1 1 1] Forward & Reverse
  (if (not (Variables|Default|GetBraking))
    (Variables|Default|SetThrottleInput AxisValue)))

(fn ConstructionScript
  (bind _headlights (Variables|Default|GetHeadlights))
  (Variables|Camera|SetCameraLength (Variables|/Script/Engine.SpringArmComponent|GetTargetArmLength (Variables|Default|GetSpringArm)))
  (if (Variables|Default|GetTorch_On)
    (Rendering|SetVisibility _headlights true true)
    (else
      (Rendering|SetVisibility _headlights false true))))

(fn ToggleTorch
  (bind _headlights_off (Variables|Default|GetHeadlights_Off))
  (bind _headlights (Variables|Default|GetHeadlights))
  (if (Variables|Default|GetTorch_On)
    (Rendering|SetVisibility _headlights false true)
    (Variables|Default|SetTorch_On false)
    (Rendering|SetVisibility _headlights_off true true)
    (else
      (Rendering|SetVisibility _headlights true true)
      (Variables|Default|SetTorch_On true)
      (Rendering|SetVisibility _headlights_off false true))))

(event Input|ActionEvents|InputActionIncrease_Speed
  (params (Key :type Key%20Structure))
  (:Pressed
    (Variables|Camera|SetCameraLength (Math|Float|Clamp(Float) (* (Variables|Camera|GetCameraLength) 0.9) 5e+02 4e+03))))

(event Input|ActionEvents|InputActionDecrease_Speed
  (params (Key :type Key%20Structure))
  (:Pressed
    (Variables|Camera|SetCameraLength (Math|Float|Clamp(Float) (* (Variables|Camera|GetCameraLength) 1.1) 5e+02 4e+03))))

(event Input|AxisEvents|InputAxisTurn
  (params (AxisValue :type Float%20%28single-precision%29))
  (if (Variables|Default|GetFirstPersonCamera)
    (Transformation|AddRelativeRotation (Variables|Default|GetSpringArmFirstPerson) (Math|Rotator|MakeRotator 0.0 0.0 (* AxisValue (Variables|Input|GetTurnRate))) false false)
    (else
      (Transformation|AddRelativeRotation (Variables|Default|GetSpringArm) (Math|Rotator|MakeRotator 0.0 0.0 (* AxisValue (Variables|Input|GetTurnRate))) false false))))

(event Input|AxisEvents|InputAxisLookUp
  (params (AxisValue :type Float%20%28single-precision%29))
  (if (Variables|Default|GetFirstPersonCamera)
    (Transformation|AddRelativeRotation (Variables|Default|GetSpringArmFirstPerson) (Math|Rotator|MakeRotator 0.0 (* (* AxisValue -1.0) (Variables|Input|GetLookUpRate)) 0.0) false false)
    (else
      (Transformation|AddRelativeRotation (Variables|Default|GetSpringArm) (Math|Rotator|MakeRotator 0.0 (* (* AxisValue -1.0) (Variables|Input|GetLookUpRate)) 0.0) false false))))

(event Input|KeyboardEvents|C
  (params (Key :type Key%20Structure))
  ;[1 1 1] Switch Camera
  (:Pressed
    (|SwitchCameraMode)))