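; Game mode Blueprint for ChooseGame that handles mouse-driven placement previews for buildings.
; TryBuild spawns the given building class at the deprojected cursor position, stores it as ItemToBeBuild and sets IsBuilding.
; While that flag is set, Tick line-traces from the cursor against WorldStatic objects with debug drawing and teleports the building to the hit point.
; The graph has no step to confirm or cancel placement.
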(event Custom|TryBuild
  (params (building :type Actor%20Class%20Reference))
  (bind _returnvalue (Game|SpawnActorfromClass building (Math|Conversions|ToTransform(Vector) (.WorldLocation (Game|Player|ConvertMouseLocationToWorldSpace (Game|GetPlayerController 0)))) "AlwaysSpawn" 0 0))
  (Variables|Default|SetitemToBeBuild _returnvalue)
  (Variables|Default|SetisBuilding true))

(event EventBeginPlay)

(event EventTick
  (params (DeltaSeconds :type Float%20%28single-precision%29))
  (bind _returnvalue (Game|GetPlayerController 0))
  (bind (_worldlocation _worlddirection) (Game|Player|ConvertMouseLocationToWorldSpace _returnvalue))
  (if (Variables|Default|GetisBuilding)
    (bind (_outhit _returnvalue_2) (Collision|LineTraceForObjects _worldlocation (+ _worldlocation (* _worlddirection 10000)) (Utilities|Array|MakeArray "ObjectTypeQuery1") false 0 "ForDuration"))
    (if _returnvalue_2
      (Transformation|SetActorTransform (Variables|Default|GetitemToBeBuild) (Math|Conversions|ToTransform(Vector) (.Location (Collision|BreakHitResult _outhit))) false true))))

(fn ConstructionScript)