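; Player controller that handles mouse input for confirming or cancelling item placement while the game is in building mode.
; Both buttons read the IsBuilding flag on GameModeBP, so the build state lives in the game mode.
; Left click clears the flag and leaves the item in the world, while right click clears it and destroys the pending ItemToBeBuild actor.
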(event EventBeginPlay)

(event EventTick
  (params (DeltaSeconds :type Float%20%28single-precision%29)))

(event Input|MouseEvents|RightMouseButton
  (params (Key :type Key%20Structure :default "None"))
  (:Pressed
    (bind _asgame_mode_bp (Utilities|Casting|CastToGameModeBP (Game|GetGameMode)))
    (if (Variables|/Game/ChooseGame/Blueprints/GameModeBP.GameModeBP_C|GetisBuilding _asgame_mode_bp)
      (Variables|/Game/ChooseGame/Blueprints/GameModeBP.GameModeBP_C|SetisBuilding _asgame_mode_bp false)
      (Actor|DestroyActor (Variables|/Game/ChooseGame/Blueprints/GameModeBP.GameModeBP_C|GetitemToBeBuild _asgame_mode_bp)))))

(event Input|MouseEvents|LeftMouseButton
  (params (Key :type Key%20Structure :default "None"))
  (:Pressed
    (bind _asgame_mode_bp (Utilities|Casting|CastToGameModeBP (Game|GetGameMode)))
    (if (Variables|/Game/ChooseGame/Blueprints/GameModeBP.GameModeBP_C|GetisBuilding _asgame_mode_bp)
      (Variables|/Game/ChooseGame/Blueprints/GameModeBP.GameModeBP_C|SetisBuilding _asgame_mode_bp false))))

(fn ConstructionScript)