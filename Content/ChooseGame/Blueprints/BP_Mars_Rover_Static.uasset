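; BP_Mars_Rover_Static is a non-animated Mars rover prop with configurable lighting, set up entirely in the Construction Script.
; A dynamic material instance on the body sets the baked glow strength from a variable.
; Booleans swap headlight on/off components and toggle tail-light point lights, with small tail-light meshes getting an off material when disabled.
; Large tail-light meshes receive the off material regardless of their flag; the event graph is unused.
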(event EventBeginPlay)

(event Collision|EventActorBeginOverlap
  (params (OtherActor :type Actor%20Object%20Reference)))

(event EventTick
  (params (DeltaSeconds :type Float%20%28single-precision%29)))

(fn ConstructionScript
  (bind _sm_marsrover_body (Variables|Default|GetSM_MarsRover_Body))
  (bind _pointlight_taillight_large_l (Variables|Default|GetPointLight%20TailLight_Large_L))
  (bind _headlights_off (Variables|Default|GetHeadlights_Off))
  (bind _headlights_on (Variables|Default|GetHeadlights_On))
  (bind _pointlight1 (Variables|Default|GetPointLight1))
  (bind _returnvalue (Rendering|Material|CreateDynamicMaterialInstance _sm_marsrover_body 0 "/Game/ChooseGame/Materials/Rover/MI_Mars_Rover_A_BakedGlow.MI_Mars_Rover_A_BakedGlow" "None" :!class /Script/Engine.PrimitiveComponent))
  (bind _output_get (Variables|Default|SetMaterial _returnvalue))
  (Rendering|Material|SetMaterial _sm_marsrover_body 0 _output_get)
  (Rendering|Material|SetScalarParameterValue (Variables|Default|GetMaterial) "Glow_Baked" (Variables|Default|GetBaked_GlowLight_Value) :!class /Script/Engine.MaterialInstanceDynamic)
  (if (Variables|Default|GetHeadlights)
    (Rendering|SetVisibility _headlights_on true true)
    (Rendering|SetVisibility _headlights_off false true)
    (else
      (Rendering|SetVisibility _headlights_on false true)
      (Rendering|SetVisibility _headlights_off true true)))
  (if (Variables|Default|GetTailLights)
    (Rendering|SetVisibility _pointlight1 true true)
    (else
      (Rendering|SetVisibility _pointlight1 false false)
      (Rendering|Material|SetMaterial (Variables|Default|GetSM_TailLight_L) 0 "/Game/ChooseGame/Materials/Rover/M_Mars_Rover_LightOff.M_Mars_Rover_LightOff")))
  (if (Variables|Default|GetTailLights_Large)
    (Rendering|SetVisibility _pointlight_taillight_large_l true true)
    (else
      (Rendering|SetVisibility _pointlight_taillight_large_l false false)))
  (Rendering|Material|SetMaterial (Variables|Default|GetTailLight_Large_R) 0 "/Game/ChooseGame/Materials/Rover/M_Mars_Rover_LightOff.M_Mars_Rover_LightOff"))