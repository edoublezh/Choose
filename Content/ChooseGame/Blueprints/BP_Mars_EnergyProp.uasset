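; BP_Mars_EnergyProp is an animated Mars energy prop built around five spinning cylinder meshes.
; The construction script gives each cylinder a random starting yaw.
; Tick then adds a per-cylinder yaw step every frame, without delta-time scaling, so spin rate depends on frame rate.
; The step is the Speed input squared, so cylinders given negative speeds turn in the same direction as the others.
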(event EventBeginPlay)

(event Collision|EventActorBeginOverlap
  (params (OtherActor :type Actor%20Object%20Reference)))

(event EventTick
  (params (DeltaSeconds :type Float%20%28single-precision%29))
  (Utilities|RotateCylinder (Variables|Default|GetSM_MARS_Block02_Energy_Cylinder1) 1.0)
  (Utilities|RotateCylinder (Variables|Default|GetSM_MARS_Block02_Energy_Cylinder2) -1.5)
  (Utilities|RotateCylinder (Variables|Default|GetSM_MARS_Block02_Energy_Cylinder3) 1.0)
  (Utilities|RotateCylinder (Variables|Default|GetSM_MARS_Block02_Energy_Cylinder4) -1.7)
  (Utilities|RotateCylinder (Variables|Default|GetSM_MARS_Block02_Energy_Cylinder5) 1.2))

(fn ConstructionScript
  (Utilities|RandomizeRotation (Variables|Default|GetSM_MARS_Block02_Energy_Cylinder1))
  (Utilities|RandomizeRotation (Variables|Default|GetSM_MARS_Block02_Energy_Cylinder2))
  (Utilities|RandomizeRotation (Variables|Default|GetSM_MARS_Block02_Energy_Cylinder3))
  (Utilities|RandomizeRotation (Variables|Default|GetSM_MARS_Block02_Energy_Cylinder4))
  (Utilities|RandomizeRotation (Variables|Default|GetSM_MARS_Block02_Energy_Cylinder5)))